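; BP_BlockDistrauctable is a destructible block that may drop a random bonus when it breaks.
; Each actor overlap decrements HintCount, with no filtering on the overlapping actor, and the block destroys itself when the count reaches zero.
; Before destruction, a weighted random roll using BPBonusCreator's Chance decides whether to spawn a class from GetRandomBonus at the Cube's world location.
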(event `self.ReceiveBeginPlay`)

(event `self.ReceiveActorBeginOverlap`
  (params (OtherActor :type "Actor Object Reference"))
  (bind _output_get (set `self.HintCount` (- (`self.HintCount`) 1)))
  (if (== _output_get 0)
    (if (`KismetMathLibrary.RandomBoolWithWeight` (`/Game/Blueprints/BP_BonusCreator.Chance` (`self.BP_BonusCreator`)))
      (bind _outitem (`/Game/Blueprints/BP_BonusCreator.GetRandomBonus` (`self.BP_BonusCreator`)))
      (`|SpawnActorFromClass` _outitem (`KismetMathLibrary.Conv_VectorToTransform` (`SceneComponent.K2_GetComponentLocation` (`self.Cube`))) "Undefined" "MultiplyWithRoot" null null))
    (`self.K2_DestroyActor`)))

(fn `UserConstructionScript`)
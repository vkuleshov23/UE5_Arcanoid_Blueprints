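; BP_Panel is a player paddle that moves sideways and spawns a BP_Ball that respawns.
; MoveRight input applies swept offsets, stepping back when it hits anything other than the ball.
; BeginPlay spawns the ball at the Capsule's location, sets its speeds and binds to its OnDead event for respawning.
; ScaleUp widens the Cube along Y in multiplicative steps until ScaleTimes is reached.
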(event `InputAxis|MoveRight`
  (params (AxisValue :type "Float (single-precision)"))
  (if (< AxisValue 0.0)
    (bind _sweephitresult (`self.K2_AddActorWorldOffset` (`self.left`) true))
    (bind (_bblockinghit _binitialoverlap _time _distance _location _impactpoint _normal _impactnormal _physmat _hitactor) (`GameplayStatics.BreakHitResult` _sweephitresult))
    (if _bblockinghit
      (cast `/Game/Blueprints/BP_Ball` _hitactor
        (:`CastFailed`
          (`self.K2_AddActorWorldOffset` (`self.right`) true))))))

(event `InputAxis|MoveRight`
  (params (AxisValue :type "Float (single-precision)"))
  (if (> AxisValue 0.0)
    (bind _sweephitresult (`self.K2_AddActorWorldOffset` (`self.right`) true))
    (bind (_bblockinghit _binitialoverlap _time _distance _location _impactpoint _normal _impactnormal _physmat _hitactor) (`GameplayStatics.BreakHitResult` _sweephitresult))
    (if _bblockinghit
      (cast `/Game/Blueprints/BP_Ball` _hitactor
        (:`CastFailed`
          (`self.K2_AddActorWorldOffset` (`self.left`) true))))))

(event `self.ReceiveBeginPlay`
  (`self.CreateRespawnableBall`))

(fn `CreateRespawnableBall`
  (bind _outputpin (`self.SpawnBall` "/Game/Blueprints/BP_Ball.BP_Ball_C"))
  (`self.SetBindToRespawn` _outputpin))

(fn `ScaleUp`
  (bind _cube (`self.Cube`))
  (bind (_returnvalue_location _returnvalue_rotation _returnvalue_scale) (`KismetMathLibrary.BreakTransform` (`SceneComponent.K2_GetComponentToWorld` _cube)))
  (if (not (== (`self.scaleTimes`) (`self.scaleUpAlreadyTimes`)))
    (`/Engine/EditorBlueprintResources/StandardMacros.IncrementInt` (`self.scaleUpAlreadyTimes`)
      (:`  `
        (`SceneComponent.SetWorldScale3D` _cube (* _returnvalue_scale (1.0 1.1 1.0)))))))

(fn `SetBindToRespawn`
  (params (Ball :type "/Game/Blueprints/BP_Ball Object Reference"))
  (add `/Game/Blueprints/BP_Ball.OnDead` Ball (`|CreateDelegate` :!event `CreateRespawnableBall`)))

(fn `SpawnBall`
  (params (Ball :type "/Game/Blueprints/BP_Ball Class Reference"))
  (returns (OutputPin :type "/Game/Blueprints/BP_Ball Object Reference"))
  (bind _returnvalue (`|SpawnActorFromClass` Ball (`KismetMathLibrary.Conv_VectorToTransform` (`SceneComponent.K2_GetComponentLocation` (`self.Capsule`))) "AlwaysSpawn" "MultiplyWithRoot" null null))
  (bind _output_get (set `self.ball` _returnvalue))
  (set `/Game/Blueprints/BP_Ball.MinSpeed` 1000.0 _output_get)
  (set `/Game/Blueprints/BP_Ball.Speed` 1500.0 _output_get)
  (set `/Game/Blueprints/BP_Ball.CurSpeed` 1500.0 _output_get)
  (return _output_get))

(fn `UserConstructionScript`)
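; BP_BlockColored is a block actor that changes color the first time another actor overlaps it.
; On overlap it calls the parent handler, then flips a boolean guard and swaps the first material slot on its Cube component.
; The guard makes the change one-way, and the overlapping actor's type is not checked.
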(event `self.ReceiveActorBeginOverlap`
  (params (OtherActor :type "Actor Object Reference"))
  (`parent.ReceiveActorBeginOverlap` OtherActor)
  (if (not (`self.isClolred`))
    (set `self.isClolred` (not (`self.isClolred`)))
    (`PrimitiveComponent.SetMaterial` (`self.Cube`) 0 "/DatasmithContent/Materials/AliasReference.AliasReference")))

(fn `UserConstructionScript`
  (`parent.UserConstructionScript`))